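; End-zone actor that decides victory or defeat when the player's helicopter character enters its box.
; On the first valid overlap only, it compares the character's VitesseGrav to VitesseLimit: above the limit is a landing, otherwise death.
; Either outcome prints a message, tints the helicopter green or red, sets SiTouche, calls FakeCollision and shows the matching end-screen HUD.
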(event `self.Box.OnComponentBeginOverlap`
  (params (OverlappedComponent :type "PrimitiveComponent Object Reference") (OtherActor :type "Actor Object Reference") (OtherComp :type "PrimitiveComponent Object Reference") (OtherBodyIndex :type Integer) (bFromSweep :type Boolean) (SweepResult :type "HitResult Structure (by ref)"))
  (bind _returnvalue (`GameplayStatics.GetPlayerCharacter` 0))
  (bind _ref_charactere (`self.REF_charactere`))
  (bind `_hélico` (`/Game/ALL/BluePrint/BP_caractere.hélico` _ref_charactere))
  ;[0.6105 0.5271 1 0.502] condition de victoire et de défet een fonction de la vitesse
  (if (== OtherActor _returnvalue)
    (bind _asbp_caractere (cast `/Game/ALL/BluePrint/BP_caractere` _returnvalue))
    (bind _output_get (set `self.REF_charactere` _asbp_caractere))
    (`/Engine/EditorBlueprintResources/StandardMacros.DoOnce` false
      (:`Completed`
        (if (> (`/Game/ALL/BluePrint/BP_caractere.vitesse_grav` _output_get) (`/Game/ALL/BluePrint/BP_caractere.Vitesse_limit` _output_get))
          (`KismetSystemLibrary.PrintString` "Vous avez atterri.")
          (`PrimitiveComponent.SetMaterial` `_hélico` 0 "/Game/ALL/Mat/Mat_green.Mat_green")
          (set `/Game/ALL/BluePrint/BP_caractere.si_touche` true _ref_charactere)
          (`/Game/ALL/BluePrint/BP_caractere. fake_collision` _ref_charactere)
          (bind _returnvalue_2 (`|GenericCreateObject` "/Game/ALL/HUD/HUD_fin_vie.HUD_fin_vie_C"))
          (bind _output_get_2 (set `self.NewVar_0` _returnvalue_2))
          (`UserWidget.AddToViewport` _output_get_2 0)
          (else
            (`KismetSystemLibrary.PrintString` "Vous avez péri !")
            (`PrimitiveComponent.SetMaterial` `_hélico` 0 "/Game/ALL/Mat/Mat_red.Mat_red")
            (set `/Game/ALL/BluePrint/BP_caractere.si_touche` true _ref_charactere)
            (`/Game/ALL/BluePrint/BP_caractere. fake_collision` _ref_charactere)
            (bind _returnvalue_3 (`|GenericCreateObject` "/Game/ALL/HUD/HUD_fin_mort.HUD_fin_mort_C"))
            (bind _output_get_3 (set `self.NewVar` _returnvalue_3))
            (`UserWidget.AddToViewport` _output_get_3 0)))))))

(fn `UserConstructionScript`)