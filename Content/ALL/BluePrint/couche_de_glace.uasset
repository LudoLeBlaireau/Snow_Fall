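; Snow/ice layer obstacle that kills the player on contact and melts while they stay in its detection zone.
; Touching Box1 turns the helicopter red, flags the hit, pauses the game and shows the death HUD.
; Zone entry starts a 0.016s looping timer that shrinks the cube's Z scale, lowering it, the zone and snow particles to compensate.
; Exiting halts melting via a flag; below a scale threshold the actor destroys itself.
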(event `self.Box1.OnComponentBeginOverlap`
  (params (OverlappedComponent :type "PrimitiveComponent Object Reference") (OtherActor :type "Actor Object Reference") (OtherComp :type "PrimitiveComponent Object Reference") (OtherBodyIndex :type Integer) (bFromSweep :type Boolean) (SweepResult :type "HitResult Structure (by ref)"))
  (bind _returnvalue (`GameplayStatics.GetPlayerCharacter` 0))
  (bind _as_bp_caractere (`self.As BP Caractere`))
  ;[0.6105 0.5271 1 0.502] si le joueur touche le block de neige, il meur
  (if (== OtherActor _returnvalue)
    (bind _asbp_caractere (cast `/Game/ALL/BluePrint/BP_caractere` _returnvalue))
    (set `self.As BP Caractere` _asbp_caractere)
    (`/Engine/EditorBlueprintResources/StandardMacros.DoOnce` false
      (:`Completed`
        (`KismetSystemLibrary.PrintString` "Vous avez péri !")
        (`PrimitiveComponent.SetMaterial` (`/Game/ALL/BluePrint/BP_caractere.hélico` _as_bp_caractere) 0 "/Game/ALL/Mat/Mat_red.Mat_red")
        (set `/Game/ALL/BluePrint/BP_caractere.si_touche` true _as_bp_caractere)
        (`/Game/ALL/BluePrint/BP_caractere. fake_collision` _as_bp_caractere)
        (`GameplayStatics.SetGamePaused` true)
        (bind _returnvalue_2 (`|CreateWidget` "/Game/ALL/HUD/HUD_fin_mort.HUD_fin_mort_C"))
        (bind _output_get (set `self.NewVar_1` _returnvalue_2))
        (`UserWidget.AddToViewport` _output_get 0)))))

(event `self.zone_detection.OnComponentEndOverlap`
  (params (OverlappedComponent :type "PrimitiveComponent Object Reference") (OtherActor :type "Actor Object Reference") (OtherComp :type "PrimitiveComponent Object Reference") (OtherBodyIndex :type Integer))
  ;[0.6105 0.5271 1 0.502] si le joueur n'est plus dans la collision box, alors la diminution du block est stoppé
  (if (== OtherActor (`GameplayStatics.GetPlayerCharacter` 0))
    (set `self.est dedans` false)))

(event `self.zone_detection.OnComponentBeginOverlap`
  (params (OverlappedComponent :type "PrimitiveComponent Object Reference") (OtherActor :type "Actor Object Reference") (OtherComp :type "PrimitiveComponent Object Reference") (OtherBodyIndex :type Integer) (bFromSweep :type Boolean) (SweepResult :type "HitResult Structure (by ref)"))
  ;[0.6105 0.5271 1 0.502] permet de détécter le joueur, si il est détéqueter, ca lance une boucle qui fait "fondre" progressivement le cube et le détruit a un certain seuil.
  ;;[1 0.6584 0.807 0.502] permet de détécter si le joueur rentre dans la zone de détection
  (if (== OtherActor (`GameplayStatics.GetPlayerCharacter` 0))
    (set `self.est dedans` true)
    (bind _returnvalue (`KismetSystemLibrary.K2_SetTimerDelegate` (delegate `tzqt`) 0.016 true))))

(event `tzqt`
  (bind _particule_de_neige (`self.particule_de_neige`))
  (bind _zone_detection (`self.zone_detection`))
  (bind _cube (`self.Cube`))
  (bind _cube_2 (`self.Cube`))
  (bind (_returnvalue_x _returnvalue_y _returnvalue_z) (`KismetMathLibrary.BreakVector` (`SceneComponent.K2_GetComponentLocation` _particule_de_neige)))
  (bind (_returnvalue_x_2 _returnvalue_y_2 _returnvalue_z_2) (`KismetMathLibrary.BreakVector` (`SceneComponent.K2_GetComponentScale` (`self.Cube`))))
  (bind (_returnvalue_x_3 _returnvalue_y_3 _returnvalue_z_3) (`KismetMathLibrary.BreakVector` (`SceneComponent.K2_GetComponentLocation` _zone_detection)))
  (bind (_returnvalue_x_4 _returnvalue_y_4 _returnvalue_z_4) (`KismetMathLibrary.BreakVector` (`SceneComponent.K2_GetComponentScale` _cube)))
  (bind (_returnvalue_x_5 _returnvalue_y_5 _returnvalue_z_5) (`KismetMathLibrary.BreakVector` (`SceneComponent.K2_GetComponentLocation` _cube_2)))
  ;[0.6105 0.5271 1 0.502] permet de détécter le joueur, si il est détéqueter, ca lance une boucle qui fait "fondre" progressivement le cube et le détruit a un certain seuil.
  ;;[1 0.6584 0.807 0.502] si le joueur est détecter, lance une opération, soit fait fondre le block, soit le détruit
  (if (`self.est dedans`)
    (if (< _returnvalue_z_2 0.5)
      ;;[1 0.6584 0.807 0.502] "détruit" le timer et détruit la neige
      (`KismetSystemLibrary.K2_ClearAndInvalidateTimerHandle` (stale `self.zone_detection.OnComponentBeginOverlap` _returnvalue))
      (`self.K2_DestroyActor`)
      (else
        (`ActorComponent.Activate` (`self.particule_de_neige`) false)
        ;;[1 0.6584 0.807 0.502] descent le block pour contrer le fait que le cube retrécit des 2 coté en meme temps, et le fx pour faire suivre ainsi que la zone de détection
        (`SceneComponent.SetWorldScale3D` _cube (`KismetMathLibrary.VInterpTo_Constant` (`KismetMathLibrary.MakeVector` _returnvalue_x_4 _returnvalue_y_4 _returnvalue_z_4) (`KismetMathLibrary.MakeVector` _returnvalue_x_4 _returnvalue_y_4 (* _returnvalue_z_4 -1.0)) (`GameplayStatics.GetWorldDeltaSeconds`) 2.0))
        (`SceneComponent.K2_SetWorldLocation` _cube_2 (`KismetMathLibrary.MakeVector` _returnvalue_x_5 _returnvalue_y_5 (- _returnvalue_z_5 2.0)) false false)
        (`SceneComponent.K2_SetWorldLocation` _particule_de_neige (`KismetMathLibrary.MakeVector` _returnvalue_x _returnvalue_y (- _returnvalue_z 4.8)) false false)
        (`SceneComponent.K2_SetWorldLocation` _zone_detection (`KismetMathLibrary.MakeVector` _returnvalue_x_3 _returnvalue_y_3 (- _returnvalue_z_3 2.0)) false false)))))

(fn `UserConstructionScript`)