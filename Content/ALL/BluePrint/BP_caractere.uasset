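; Player-controlled helicopter that falls under simulated gravity and climbs on a fuel-limited thrust button.
; A looping timer lowers a clamped vertical speed and updates the HUD altimeter relative to a TargetPoint, with pause and unpause calls on button press and release.
; Holding thrust burns fuel, updates the HUD and raises that speed, which Tick applies directly to world Z.
; A fake collision event zeroes speed and pauses the game when touched.
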(event `self.ReceivePossessed`
  (params (NewController :type "Controller Object Reference"))
  ;[0.6105 0.5271 1 0.502] permet d'utiliser les input de IMC_base
  (if (`Controller.IsPlayerController` NewController)
    (bind _asplayer_controller (cast `PlayerController` NewController))
    (`EnhancedInputSubsystemInterface.AddMappingContext` (pcsubsystem `EnhancedInputLocalPlayerSubsystem` _asplayer_controller) "/Game/ALL/Base/IMC_base.IMC_base" 0 (struct))))

(event `fake_collision`
  ;[0.6105 0.5271 1 0.502] créé une fausse collision
  (if (`self.si_touche`)
    (set `self.vitesse_grav` 0.0)
    (`GameplayStatics.SetGamePaused` true)))

(event `self.ReceiveBeginPlay`
  (`/Engine/EditorBlueprintResources/StandardMacros.DoOnce` false
    (:`Completed`
      (bind _returnvalue (`|GenericCreateObject` "/Game/ALL/HUD/HUD_new.HUD_new_C"))
      (bind _output_get (set `self.As HUD Progress` _returnvalue))
      ;[0.6105 0.5271 1 0.502] Comment
      (`UserWidget.AddToViewport` _output_get 0)
      (bind _returnvalue_2 (`KismetSystemLibrary.K2_SetTimerDelegate` (delegate `timer grav`) 0.016667 true true))
      (set `self.Timer gravity` _returnvalue_2))))

(event `timer grav`
  (bind (_returnvalue_x _returnvalue_y _returnvalue_z) (`KismetMathLibrary.BreakVector` (`SceneComponent.K2_GetComponentLocation` (`self.hélico`))))
  ;[0.6105 0.5271 1 0.502] Comment
  ;;[1 0.6584 0.807 0.502] si le timer est en ON: alors set la graviter en négatif pour faire chuter l'objet
  (if (not (`self.si_touche`))
    (set `self.vitesse_grav` (`KismetMathLibrary.FClamp` (+ (`self.vitesse_grav`) -1.55) -100.0 100.0))
    (bind _returnvalue (`GameplayStatics.GetActorOfClass` "/Script/Engine.TargetPoint"))
    (bind (_returnvalue_x_2 _returnvalue_y_2 _returnvalue_z_2) (`KismetMathLibrary.BreakVector` (`SceneComponent.K2_GetComponentLocation` (`TargetPoint.ArrowComponent` _returnvalue))))
    (bind _output_get (set `self.Altitude` (* (- _returnvalue_z_2 _returnvalue_z) -1.0)))
    (`/Game/ALL/HUD/HUD_new.altimetre` (`self.As HUD Progress`) (`KismetMathLibrary.FTrunc` _output_get))))

(event `EnhancedInput|/Game/ALL/Base/IA_button`
  (params (ActionValue :type Boolean) (ElapsedSeconds :type "Float (double-precision)") (TriggeredSeconds :type "Float (double-precision)") (InputAction :type "InputAction Object Reference" :default "/Game/ALL/Base/IA_button.IA_button"))
  ;[0.6105 0.5271 1 0.502] gestion de la propulsion de l'objet pour "inversser" la graviter
  (:`Triggered`
    ;;[1 0.6584 0.807 0.502] vérifie si le joueur est posé
    (if (not (`self.si_touche`))
      ;;[1 0.6584 0.807 0.502] set la barre de carburant et l'affiche
      (if (> (`self.Carbu`) 0.0)
        (bind _output_get (set `self.Carbu` (- (`self.Carbu`) (`self.perte_carbu`))))
        (`/Game/ALL/HUD/HUD_new.Carbu_descente` (`self.As HUD Progress`) _output_get)
        ;;[1 0.6584 0.807 0.502] set la graviter pour la remonter
        (set `self.vitesse_grav` (`KismetMathLibrary.FClamp` (+ (`self.vitesse_grav`) 2.5) -100.0 100.0)))))
  (:`Started`
    ;;[1 0.6584 0.807 0.502] if click: timer pause, else timer on
    (set `self.Timer gravity` (struct))
    (`KismetSystemLibrary.K2_PauseTimerHandle` (struct)))
  (:`Completed`
    (set `self.Timer gravity` (struct))
    (`KismetSystemLibrary.K2_UnPauseTimerHandle` (struct))))

(event `self.ReceiveTick`
  (params (DeltaSeconds :type "Float (single-precision)"))
  (bind `_hélico` (`self.hélico`))
  (bind (_returnvalue_x _returnvalue_y _returnvalue_z) (`KismetMathLibrary.BreakVector` (`SceneComponent.K2_GetComponentLocation` `_hélico`)))
  ;[0.6105 0.5271 1 0.502] set la position de l'object en fonction de la vitesse de graviter qui est récupérer
  (`SceneComponent.K2_SetWorldLocation` `_hélico` (`KismetMathLibrary.MakeVector` _returnvalue_x _returnvalue_y (+ _returnvalue_z (`self.vitesse_grav`))) false false))

(fn `UserConstructionScript`)