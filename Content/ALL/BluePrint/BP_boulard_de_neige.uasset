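; BP_boulard_de_neige is a snowball hazard that kills the player on touch.
; When its Sphere1 component overlaps the player character, a DoOnce prints a death message, turns the BP_caractere's Hélico mesh red, sets SiTouche and calls FakeCollision.
; It then creates the HUD_fin_mort death screen and adds it to the viewport.
; The file contains no movement logic.
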(event `self.Sphere1.OnComponentBeginOverlap`
  (params (OverlappedComponent :type "PrimitiveComponent Object Reference") (OtherActor :type "Actor Object Reference") (OtherComp :type "PrimitiveComponent Object Reference") (OtherBodyIndex :type Integer) (bFromSweep :type Boolean) (SweepResult :type "HitResult Structure (by ref)"))
  (bind _returnvalue (`GameplayStatics.GetPlayerCharacter` 0))
  (bind _ref_character (`self.REF_character`))
  ;[0.6105 0.5271 1 0.502] si le joueur touche la boule, il meurt
  (if (== OtherActor _returnvalue)
    (bind _asbp_caractere (cast `/Game/ALL/BluePrint/BP_caractere` _returnvalue))
    (set `self.REF_character` _asbp_caractere)
    (`/Engine/EditorBlueprintResources/StandardMacros.DoOnce` false
      (:`Completed`
        (`KismetSystemLibrary.PrintString` "Vous avez péri !")
        (`PrimitiveComponent.SetMaterial` (`/Game/ALL/BluePrint/BP_caractere.hélico` _ref_character) 0 "/Game/ALL/Mat/Mat_red.Mat_red")
        (set `/Game/ALL/BluePrint/BP_caractere.si_touche` true _ref_character)
        (`/Game/ALL/BluePrint/BP_caractere. fake_collision` _ref_character)
        (bind _returnvalue_2 (`|GenericCreateObject` "/Game/ALL/HUD/HUD_fin_mort.HUD_fin_mort_C"))
        (bind _output_get (set `self.NewVar` _returnvalue_2))
        (`UserWidget.AddToViewport` _output_get 0)))))

(fn `UserConstructionScript`)