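; Layered snow obstacle that the player's helicopter clears by staying in its detection zone, and that kills the player on contact.
; While the player overlaps the zone, a fast looping timer steps through a four-state enum, playing powder FX and destroying each layer after a delay, then the actor.
; Touching a layer's box triggers death once: red helicopter material, fake collision, paused game and death HUD.
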(event `self.detection_neige.OnComponentBeginOverlap`
  (params (OverlappedComponent :type "PrimitiveComponent Object Reference") (OtherActor :type "Actor Object Reference") (OtherComp :type "PrimitiveComponent Object Reference") (OtherBodyIndex :type Integer) (bFromSweep :type Boolean) (SweepResult :type "HitResult Structure (by ref)"))
  (if (== OtherActor (`GameplayStatics.GetPlayerCharacter` 0))
    (set `self.est_dedant` true)
    (`KismetSystemLibrary.K2_SetTimerDelegate` (delegate `elevage_de_couche_si_dedant`) 0.036 true)))

(event `elevage_de_couche_si_dedant`
  (if (`self.est_dedant`)
    (switch `/Game/ALL/BluePrint/sert_plus_mais_utile/ENUM_select_couche` (`self.ENUM_select_couche`)
      (:`NewEnumerator0`
        (`ActorComponent.Activate` (`self.FX_poudre_de_neige_1`) false)
        (`KismetSystemLibrary.Delay` 2.0)
        (`ActorComponent.K2_DestroyComponent` (`self.1ere_couche`))
        (`ActorComponent.K2_DestroyComponent` (`self.Box_1`))
        (`ActorComponent.K2_DestroyComponent` (`self.FX_poudre_de_neige_1`))
        (set `self.ENUM_select_couche` "NewEnumerator1"))
      (:`NewEnumerator1`
        (`ActorComponent.Activate` (`self.FX_poudre_de_neige_2`) false)
        (`KismetSystemLibrary.Delay` 2.0)
        (`ActorComponent.K2_DestroyComponent` (`self.2eme_couche`))
        (`ActorComponent.K2_DestroyComponent` (`self.Box_2`))
        (`ActorComponent.K2_DestroyComponent` (`self.FX_poudre_de_neige_2`))
        (set `self.ENUM_select_couche` "NewEnumerator2"))
      (:`NewEnumerator2`
        (`ActorComponent.Activate` (`self.FX_poudre_de_neige_3`) false)
        (`KismetSystemLibrary.Delay` 2.0)
        (`ActorComponent.K2_DestroyComponent` (`self.3eme_couche`))
        (`ActorComponent.K2_DestroyComponent` (`self.Box_3`))
        (`ActorComponent.K2_DestroyComponent` (`self.FX_poudre_de_neige_3`))
        (set `self.ENUM_select_couche` "NewEnumerator3"))
      (:`NewEnumerator3`
        (`ActorComponent.Activate` (`self.FX_poudre_de_neige_4`) false)
        (`KismetSystemLibrary.Delay` 2.0)
        (`self.K2_DestroyActor`)))))

(event `self.ReceiveBeginPlay`
  (set `self.ENUM_select_couche` "NewEnumerator0"))

(event `self.detection_neige.OnComponentEndOverlap`
  (params (OverlappedComponent :type "PrimitiveComponent Object Reference") (OtherActor :type "Actor Object Reference") (OtherComp :type "PrimitiveComponent Object Reference") (OtherBodyIndex :type Integer))
  (if (== OtherActor (`GameplayStatics.GetPlayerCharacter` 0))
    (set `self.est_dedant` false)))

(event `self.Box_4.OnComponentBeginOverlap`
  (params (OverlappedComponent :type "PrimitiveComponent Object Reference") (OtherActor :type "Actor Object Reference") (OtherComp :type "PrimitiveComponent Object Reference") (OtherBodyIndex :type Integer) (bFromSweep :type Boolean) (SweepResult :type "HitResult Structure (by ref)"))
  (bind _returnvalue (`GameplayStatics.GetPlayerCharacter` 0))
  (bind _as_bp_caractere (`self.As BP Caractere`))
  ; couche 1
  (if (== OtherActor _returnvalue)
    (bind _asbp_caractere (cast `/Game/ALL/BluePrint/BP_caractere` _returnvalue))
    (set `self.As BP Caractere_0` _asbp_caractere)
    (`/Engine/EditorBlueprintResources/StandardMacros.DoOnce` false
      (:`Completed`
        (`KismetSystemLibrary.PrintString` "Vous avez péri !")
        (`PrimitiveComponent.SetMaterial` (`/Game/ALL/BluePrint/BP_caractere.hélico` _as_bp_caractere) 0 "/Game/ALL/Mat/Mat_red.Mat_red")
        (set `/Game/ALL/BluePrint/BP_caractere.si_touche` true _as_bp_caractere)
        (`/Game/ALL/BluePrint/BP_caractere. fake_collision` _as_bp_caractere)
        (`GameplayStatics.SetGamePaused` true)
        (bind _returnvalue_2 (`|GenericCreateObject` "/Game/ALL/HUD/HUD_fin_mort.HUD_fin_mort_C"))
        (bind _output_get (set `self.NewVar` _returnvalue_2))
        (`UserWidget.AddToViewport` _output_get 0)))))

(event `self.Box_3.OnComponentBeginOverlap`
  (params (OverlappedComponent :type "PrimitiveComponent Object Reference") (OtherActor :type "Actor Object Reference") (OtherComp :type "PrimitiveComponent Object Reference") (OtherBodyIndex :type Integer) (bFromSweep :type Boolean) (SweepResult :type "HitResult Structure (by ref)"))
  (bind _returnvalue (`GameplayStatics.GetPlayerCharacter` 0))
  (bind _as_bp_caractere (`self.As BP Caractere`))
  ; couche 2
  (if (== OtherActor _returnvalue)
    (bind _asbp_caractere (cast `/Game/ALL/BluePrint/BP_caractere` _returnvalue))
    (set `self.As BP Caractere_0` _asbp_caractere)
    (`/Engine/EditorBlueprintResources/StandardMacros.DoOnce` false
      (:`Completed`
        (`KismetSystemLibrary.PrintString` "Vous avez péri !")
        (`PrimitiveComponent.SetMaterial` (`/Game/ALL/BluePrint/BP_caractere.hélico` _as_bp_caractere) 0 "/Game/ALL/Mat/Mat_red.Mat_red")
        (set `/Game/ALL/BluePrint/BP_caractere.si_touche` true _as_bp_caractere)
        (`/Game/ALL/BluePrint/BP_caractere. fake_collision` _as_bp_caractere)
        (`GameplayStatics.SetGamePaused` true)
        (bind _returnvalue_2 (`|GenericCreateObject` "/Game/ALL/HUD/HUD_fin_mort.HUD_fin_mort_C"))
        (bind _output_get (set `self.NewVar` _returnvalue_2))
        (`UserWidget.AddToViewport` _output_get 0)))))

(event `self.Box_2.OnComponentBeginOverlap`
  (params (OverlappedComponent :type "PrimitiveComponent Object Reference") (OtherActor :type "Actor Object Reference") (OtherComp :type "PrimitiveComponent Object Reference") (OtherBodyIndex :type Integer) (bFromSweep :type Boolean) (SweepResult :type "HitResult Structure (by ref)"))
  (bind _returnvalue (`GameplayStatics.GetPlayerCharacter` 0))
  (bind _as_bp_caractere (`self.As BP Caractere`))
  ; couche 3
  (if (== OtherActor _returnvalue)
    (bind _asbp_caractere (cast `/Game/ALL/BluePrint/BP_caractere` _returnvalue))
    (set `self.As BP Caractere_0` _asbp_caractere)
    (`/Engine/EditorBlueprintResources/StandardMacros.DoOnce` false
      (:`Completed`
        (`KismetSystemLibrary.PrintString` "Vous avez péri !")
        (`PrimitiveComponent.SetMaterial` (`/Game/ALL/BluePrint/BP_caractere.hélico` _as_bp_caractere) 0 "/Game/ALL/Mat/Mat_red.Mat_red")
        (set `/Game/ALL/BluePrint/BP_caractere.si_touche` true _as_bp_caractere)
        (`/Game/ALL/BluePrint/BP_caractere. fake_collision` _as_bp_caractere)
        (`GameplayStatics.SetGamePaused` true)
        (bind _returnvalue_2 (`|GenericCreateObject` "/Game/ALL/HUD/HUD_fin_mort.HUD_fin_mort_C"))
        (bind _output_get (set `self.NewVar` _returnvalue_2))
        (`UserWidget.AddToViewport` _output_get 0)))))

(event `self.Box_1.OnComponentBeginOverlap`
  (params (OverlappedComponent :type "PrimitiveComponent Object Reference") (OtherActor :type "Actor Object Reference") (OtherComp :type "PrimitiveComponent Object Reference") (OtherBodyIndex :type Integer) (bFromSweep :type Boolean) (SweepResult :type "HitResult Structure (by ref)"))
  (bind _returnvalue (`GameplayStatics.GetPlayerCharacter` 0))
  (bind _as_bp_caractere (`self.As BP Caractere`))
  ; couche 4
  (if (== OtherActor _returnvalue)
    (bind _asbp_caractere (cast `/Game/ALL/BluePrint/BP_caractere` _returnvalue))
    (set `self.As BP Caractere_0` _asbp_caractere)
    (`/Engine/EditorBlueprintResources/StandardMacros.DoOnce` false
      (:`Completed`
        (`KismetSystemLibrary.PrintString` "Vous avez péri !")
        (`PrimitiveComponent.SetMaterial` (`/Game/ALL/BluePrint/BP_caractere.hélico` _as_bp_caractere) 0 "/Game/ALL/Mat/Mat_red.Mat_red")
        (set `/Game/ALL/BluePrint/BP_caractere.si_touche` true _as_bp_caractere)
        (`/Game/ALL/BluePrint/BP_caractere. fake_collision` _as_bp_caractere)
        (`GameplayStatics.SetGamePaused` true)
        (bind _returnvalue_2 (`|GenericCreateObject` "/Game/ALL/HUD/HUD_fin_mort.HUD_fin_mort_C"))
        (bind _output_get (set `self.NewVar` _returnvalue_2))
        (`UserWidget.AddToViewport` _output_get 0)))))

(fn `UserConstructionScript`)