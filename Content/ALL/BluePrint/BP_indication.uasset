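; BP_indication is an indicator actor that shows by colour whether the player's VitesseGrav exceeds their VitesseLimit.
; When the player overlaps its Box, it caches the BP_caractere reference and starts a looping timer at a short interval.
; Each tick of the timer sets the Cube's material to green above the limit and red otherwise, with no logic to clear the timer.
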(event `self.Box.OnComponentBeginOverlap`
  (params (OverlappedComponent :type "PrimitiveComponent Object Reference") (OtherActor :type "Actor Object Reference") (OtherComp :type "PrimitiveComponent Object Reference") (OtherBodyIndex :type Integer) (bFromSweep :type Boolean) (SweepResult :type "HitResult Structure (by ref)"))
  (bind _returnvalue (`GameplayStatics.GetPlayerCharacter` 0))
  (if (== OtherActor _returnvalue)
    (bind _output_get (set `self.As BP Caractere` (cast `/Game/ALL/BluePrint/BP_caractere` _returnvalue :!pure true)))
    (`KismetSystemLibrary.K2_SetTimerDelegate` (delegate `set_color`) 0.036 true)))

(event `set_color`
  (bind _cube (`self.Cube`))
  (if (> (`/Game/ALL/BluePrint/BP_caractere.vitesse_grav` (stale `self.Box.OnComponentBeginOverlap` _output_get)) (`/Game/ALL/BluePrint/BP_caractere.Vitesse_limit` (stale `self.Box.OnComponentBeginOverlap` _output_get)))
    (`PrimitiveComponent.SetMaterial` _cube 0 "/Game/ALL/Mat/Mat_green.Mat_green")
    (else
      (`PrimitiveComponent.SetMaterial` _cube 0 "/Game/ALL/Mat/Mat_red.Mat_red"))))

(fn `UserConstructionScript`)