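; BP_generator spawns a line or a 2D grid of BP_cel actors and can remove them again.
; generate_line fills one row along X, while generationdeplaque uses nested loops over Size X and Y, spacing cells by SizeCell at a fixed height in world space.
; Both track spawned cells in AllCell, which destroyer uses to destroy every cell before clearing the array.
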(event `generate_line`
  (for _index (range (+ (`KismetMathLibrary.FTrunc` (- (`KismetMathLibrary.BreakVector2D` (`self.Size`)) 1.0)) 1))
    (bind _returnvalue (`|SpawnActorFromClass` "/Game/ALL/Pas_le_meme_projet/BP_cel.BP_cel_C" (`KismetMathLibrary.MakeTransform` (`KismetMathLibrary.MakeVector` (* _index (`self.Size_cell`)) 0.0 200.0)) "Undefined" "MultiplyWithRoot" null null))
    (`KismetArrayLibrary.Array_AddUnique` (`self.all_cell`) _returnvalue)))

(event `destroyer`
  (bind _all_cell (`self.all_cell`))
  (for _array_element _all_cell
    (`self.K2_DestroyActor` _array_element))
  (`KismetArrayLibrary.Array_Clear` _all_cell))

(event `generation de plaque`
  (for _index (range (+ (`KismetMathLibrary.FTrunc` (- (`KismetMathLibrary.BreakVector2D` (`self.Size`)) 1.0)) 1))
    (for _index_2 (range (+ (`KismetMathLibrary.FTrunc` (- (`.Y` (`KismetMathLibrary.BreakVector2D` (`self.Size`))) 1.0)) 1))
      (bind _returnvalue (`|SpawnActorFromClass` "/Game/ALL/Pas_le_meme_projet/BP_cel.BP_cel_C" (`KismetMathLibrary.MakeTransform` (`KismetMathLibrary.MakeVector` (* _index (`self.Size_cell`)) (`KismetMathLibrary.Conv_IntToDouble` (* _index_2 (`self.Size_cell`))) 200.0)) "Undefined" "MultiplyWithRoot" null null))
      (`KismetArrayLibrary.Array_AddUnique` (`self.all_cell`) _returnvalue))))

(fn `UserConstructionScript`)